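; Goal actor for the flocking system that moves continuously along a circular path in the world XZ plane.
; Each Tick advances a time counter that wraps at Period, then converts it to an angle for cosine and sine.
; The result, scaled by MoveScale, is set directly as the absolute location without sweep, so the circle centers on the world origin rather than the placed position.
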(event `self.ReceiveTick`
  (params (DeltaSeconds :type "Float (single-precision)"))
  (bind _period (`self.Period`))
  (bind _returnvalue (+ DeltaSeconds (`self.PeriodCounter`)))
  (bind _output_get (set `self.PeriodCounter` (`KismetMathLibrary.SelectFloat` _returnvalue (- _returnvalue _period) (< _returnvalue _period))))
  (bind _returnvalue_2 (* (/ _output_get _period) 360.0))
  (`self.K2_SetActorLocation` (* (`KismetMathLibrary.MakeVector` (`KismetMathLibrary.DegCos` _returnvalue_2) 0.0 (`KismetMathLibrary.DegSin` _returnvalue_2)) (`self.MoveScale`))))

(fn `UserConstructionScript`)